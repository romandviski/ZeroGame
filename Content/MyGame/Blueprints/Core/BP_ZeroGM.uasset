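; BP_ZeroGM is a game mode that spawns players and keeps their player lists current.
; Each new player possesses a randomly chosen male or female character at a random PlayerStart.
; Joins and logouts trigger a debounced list refresh on every player controller.
; ReadyToStartMatch always returns false; StartGame flags the game started and spawns everyone, but its delayed auto-start branch is disconnected.
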(event Custom|StartGame
  ;[0.5 0 0.5] Начало игры
  (Variables|Default|SetbGameStarted true)
  (for _array_element (Variables|/Script/Engine.GameStateBase|GetPlayerArray (Game|GetGameState))
    (CallFunction|SpawnPlayerCharacter (Game|GetPlayerController _array_element)))
  (CallFunction|UpdatePlayerList))

(event Custom|UpdatePlayerList
  ;[0.5 0 0.5] Новый игрок
  (Utilities|FlowControl|RetriggerableDelay 1.0)
  (for _array_element (Variables|/Script/Engine.GameStateBase|GetPlayerArray (Game|GetGameState))
    (bind _asbp_player_controller (Utilities|Casting|CastToBP_PlayerController (Game|GetPlayerController _array_element)))
    (Default|UpdatePlayerList _asbp_player_controller)))

(event EventBeginPlay)

(event EventOnLogout
  (params (ExitingController :type Controller%20Object%20Reference))
  ;[0.5 0 0.5] Игрок вышел
  (CallFunction|UpdatePlayerList))

(event EventHandleStartingNewPlayer
  (params (NewPlayer :type Player%20Controller%20Object%20Reference))
  ;[0.5 0 0.5] Новый игрок
  (CallFunction|SpawnPlayerCharacter NewPlayer)
  (CallFunction|UpdatePlayerList))

(event EventTick
  (params (DeltaSeconds :type Float%20%28single-precision%29)))

(event EventPostLogin
  (params (NewPlayer :type Player%20Controller%20Object%20Reference))
  ;[0.5 0 0.5] Новый игрок
)

(fn ConstructionScript)

(fn SpawnPlayerCharacter
  (params (PlayerController :type Player%20Controller%20Object%20Reference))
  (bind _outactors (Actor|GetAllActorsOfClass "/Script/Engine.PlayerStart"))
  (bind _aspawn (Utilities|Casting|CastToPawnClass (select (Math|Random|RandomBool) "/Game/MyGame/Blueprints/Characters/BP_MyCharacter_Girl.BP_MyCharacter_Girl_C" "/Game/MyGame/Blueprints/Characters/BP_MyCharacter.BP_MyCharacter_C"))
    (:then
      (Variables|Default|SetDefaultPawnClass _aspawn))
    (:CastFailed
      _))
  (bind _returnvalue (Game|SpawnActorfromClass (Variables|Default|GetDefaultPawnClass) (Transformation|GetActorTransform (.OutItem (Utilities|Array|Random _outactors))) "AdjustIfPossibleButAlwaysSpawn" "SelectDefaultAtRuntime" PlayerController 0))
  (Pawn|Possess PlayerController _returnvalue))

(fn ReadytoStartMatch
  (|CallParentFunction)
  (return false))