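; Player controller that owns the HUD and respawns the player's character.
; On possess, the local controller creates the HUD or resets its health display, then after a short delay binds to the character's health-change event to keep the HUD updated.
; It also forwards player list refreshes to the HUD.
; When a ZeroCharacter is unpossessed, the server waits through a retriggerable delay, then asks BP_ZeroGM to spawn a new character.
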(event Custom|UpdatePlayerList
  ;[0.5 0 0.5] Виджет при вселении
  (if (Pawn|IsLocalController)
    (bind _widget_hud (Variables|Default|GetWidget_HUD)
      (:then
        (Default|UpdatePlayerList _widget_hud))
      (:else))))

(event Custom|WidgetInit_Owning
  ;[0.5 0 0.5] Виджет при вселении
  (if (Pawn|IsLocalController)
    (Utilities|FlowControl|Sequence
      (:then_0
        (bind _widget_hud (Variables|Default|GetWidget_HUD)
          (:then
            (Default|UpdateHealth _widget_hud 1e+02))
          (:else
            (bind _returnvalue (UserInterface|CreateWidget "/Game/MyGame/UI/WBP_HUD.WBP_HUD_C" self))
            (bind _output_get (Variables|Default|SetWidget_HUD _returnvalue))
            (UserInterface|Viewport|AddtoViewport _output_get 0)
            (Input|SetInputModeGameOnly self false))))
      (:then_1
        (Utilities|FlowControl|Delay 0.2)
        (bind _asbp_my_character (Utilities|Casting|CastToBP_MyCharacter (Pawn|GetControlledPawn)))
        (EventDispatchers|BindEventtoCharacterHealthChanged _asbp_my_character (EventDispatchers|CreateEvent :!event UpdateHealthonWidget))))))

(event EventBeginPlay
  ;[0.5 0 0.5] Инпут на игру
)

(event EventPossess
  (params (PossessedPawn :type Pawn%20Object%20Reference))
  ;[0.5 0 0.5] Виджет при вселении
  (CallFunction|WidgetInitOwning))

(event EventUnPossess
  (params (UnpossessedPawn :type Pawn%20Object%20Reference))
  ;[0.5 0 0.5] При выселении
  (Utilities|Casting|CastToZeroCharacter UnpossessedPawn)
  (Networking|SwitchHasAuthority
    (:Authority
      (Utilities|FlowControl|RetriggerableDelay 5.0)
      (bind _asbp_zero_gm (Utilities|Casting|CastToBP_ZeroGM (Game|GetGameMode)))
      (Default|SpawnPlayerCharacter _asbp_zero_gm self))))

(fn ConstructionScript)

(fn UpdateHealthonWidget
  (params (CurrentHealth :type Float%20%28single-precision%29))
  (bind _widget_hud (Variables|Default|GetWidget_HUD)
    (:then
      (Default|UpdateHealth _widget_hud CurrentHealth))
    (:else)))