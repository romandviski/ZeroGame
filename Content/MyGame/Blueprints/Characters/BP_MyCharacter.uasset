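; BP_MyCharacter is a character Blueprint holding an experiment in replicating the mesh position of a dead character.
; BeginPlay and Tick only call their parent versions.
; A multicast event teleports the mesh toward a received location using a fast VInterpTo.
; The authority-side logic that would send the mesh location when HealthComponent reports not alive is disconnected, so it never runs.
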(event Custom|ReplicatePhysic_Multicast
  (params (NewLocation :type Vector))
  (bind _mesh (Variables|Character|GetMesh))
  ;[1 0 0] Просто эксперимент =)
  (Transformation|SetWorldLocation _mesh (Math|Interpolation|VInterpTo (Transformation|GetWorldLocation _mesh) NewLocation (Utilities|Time|GetWorldDeltaSeconds) 1e+03) false true))

(event EventBeginPlay
  (|CallParentFunction))

(event EventTick
  (params (DeltaSeconds :type Float%20%28single-precision%29))
  ;[1 0 0] Просто эксперимент =)
  (|CallParentFunction DeltaSeconds))

(fn ConstructionScript)